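; BP_WarningLight is a warning light actor that makes its point light flash repeatedly.
; Tick accumulates RunningTime and applies a modulo to it, switching the light between full and zero intensity for a short pulse in each cycle.
; A Delay variable is added to the time as a phase offset, shifting when the flash occurs.
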(event EventBeginPlay)

(event Collision|EventActorBeginOverlap
  (params (OtherActor :type Actor%20Object%20Reference)))

(event EventTick
  (params (DeltaSeconds :type Float%20%28single-precision%29))
  (Variables|Default|SetRunningTime (+ (Variables|Default|GetRunningTime) DeltaSeconds))
  (Rendering|Components|Light|SetIntensity (Variables|Default|GetPointLight) (Math|Float|SelectFloat 1e+04 0.0 (< (Math|Float|%(Float) (+ (Variables|Default|GetDelay) (Variables|Default|GetRunningTime)) 0.8) 0.15))))

(fn ConstructionScript)